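; BP_ConheadZombie is the conehead zombie enemy in a Plants vs. Zombies-style game, handling damage, freezing and death.
; AnyDamage passes damage to ReduceHP, which at zero HP calls DestroyZombieEvent on MyPVZGameModeBase and destroys the actor.
; Damage causers tagged Snowpea also set the Frozen flag for a few seconds.
; A walk-speed slowdown chain is left unconnected, and this graph never reads Frozen.
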(event EventBeginPlay)

(event Collision|EventActorBeginOverlap
  (params (OtherActor :type Actor%20Object%20Reference)))

(event EventTick
  (params (DeltaSeconds :type Float%20%28single-precision%29)))

(event Game|Damage|EventAnyDamage
  (params (Damage :type Float%20%28single-precision%29) (DamageType :type Damage%20Type%20Object%20Reference) (InstigatedBy :type Controller%20Object%20Reference) (DamageCauser :type Actor%20Object%20Reference))
  (Utilities|FlowControl|Sequence
    (:then_0
      (CallFunction|ReduceHP Damage))
    (:then_1
      (Utilities|IsValid DamageCauser
        (:Is%20Valid
          (if (Actor|ActorHasTag DamageCauser "Snowpea")
            (Variables|Default|SetbFrozen true)
            (Utilities|FlowControl|Delay 6.0)
            (Variables|Default|SetbFrozen false)))))))

(fn ConstructionScript)

(fn ReduceHP
  (params (Damage :type Float%20%28double-precision%29))
  (bind _output_get (Variables|Default|SetHP (- (Variables|Default|GetHP) Damage)))
  (if (<= _output_get 0.0)
    (bind _asmy_pvzgame_mode_base (Utilities|Casting|CastToMyPVZGameModeBase (Game|GetGameMode)))
    (bind _output_get_2 (Variables|Default|SetAs%20My%20PVZGame%20Mode%20Base _asmy_pvzgame_mode_base))
    (Default|DestroyZombieEvent _output_get_2)
    (Utilities|IsValid self
      (:Is%20Valid
        (Actor|DestroyActor)))))