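; Base zombie character for a Plants vs. Zombies-style game, using a flipbook sprite and capsule collision.
; Tick moves it along negative X at a Speed-scaled rate, or along its half-scaled forward vector when Frozen.
; Capsule overlap with a Deadline actor pauses the game on a lose screen with music, while a Jalapeno overlap binds BoomDeath to its bomb event.
; BoomDeath plays the explosion flipbook, then destroys the zombie and notifies the game mode.
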(event OnComponentBeginOverlap(CapsuleComponent)
  (params (OverlappedComponent :type Primitive%20Component%20Object%20Reference) (OtherActor :type Actor%20Object%20Reference) (OtherComp :type Primitive%20Component%20Object%20Reference) (OtherBodyIndex :type Integer) (bFromSweep :type Boolean) (SweepResult :type Hit%20Result%20Structure%20%28by%20ref%29))
  (Utilities|IsValid OtherActor
    (:Is%20Valid
      (Utilities|FlowControl|Sequence
        (:then_0
          (if (Actor|ActorHasTag OtherActor "Deadline")
            (Audio|PlaySound2D "/Game/Sound/losemusic_Cue.losemusic_Cue" 1.0 1.0 0.0 0 0)
            (bind _returnvalue (UserInterface|CreateWidget "/Game/Widget/Menu/Game_Lose.Game_Lose_C"))
            (UserInterface|Viewport|AddtoViewport _returnvalue 0)
            (Game|SetGamePaused true)))
        (:then_1
          (if (Actor|ActorHasTag OtherActor "MC_Jalapeno")
            (bind _asmc_jalapeno (Utilities|Casting|CastToMC_Jalapeno OtherActor))
            (EventDispatchers|BindEventtoBombDeath _asmc_jalapeno (delegate Custom|BoomDeath))))))))

(event Custom|BoomDeath
  (Sprite|SetFlipbook (Variables|Default|GetSprite) "/Game/Zombie/BoomDeath/BoomDie.BoomDie")
  (Utilities|FlowControl|Delay 1.0)
  (Utilities|IsValid self
    (:Is%20Valid
      (Actor|DestroyActor)
      (Default|CallDistroyZombie (Variables|Default|GetAs%20My%20PVZGame%20Mode%20Base_0)))))

(event EventBeginPlay
  (|CallParentFunction)
  (bind _asmy_pvzgame_mode_base (Utilities|Casting|CastToMyPVZGameModeBase (Game|GetGameMode)))
  (Variables|Default|SetAs%20My%20PVZGame%20Mode%20Base_0 _asmy_pvzgame_mode_base))

(event Collision|EventActorBeginOverlap
  (params (OtherActor :type Actor%20Object%20Reference))
  (|CallParentFunction OtherActor) ; 此节点被禁用，将不会被调用。\n从引脚连出引线来编译功能。
)

(event EventTick
  (params (DeltaSeconds :type Float%20%28single-precision%29))
  (bind _speed (Variables|Default|Getspeed))
  (bind _returnvalue (/ _speed 1.2e+04))
  (|CallParentFunction DeltaSeconds)
  (if (Variables|Default|GetbFrozen)
    (Pawn|Input|AddMovementInput (* (Transformation|GetActorForwardVector) "0.500000,0.000000,0.000000") _returnvalue false)
    (else
      (Pawn|Input|AddMovementInput "-1.000000,0.000000,0.000000" _returnvalue false))))

(fn ConstructionScript
  (|CallParentFunction))